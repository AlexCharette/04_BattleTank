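; Mortar actor Blueprint that sets up a mortar's aiming and health bar when play begins.
; BeginPlay initialises the TankAiming component with the Dome as turret and the Barrel as barrel.
; It then casts the Widget component's user widget to Healthbar_BP and passes the mortar in as that widget's Tank reference, reusing the tank aiming and health bar pieces.
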(event EventBeginPlay
  (Class|TankAimingComponent|Initialise (Variables|Default|GetTankAiming) (Variables|Default|GetDome) (Variables|Default|GetBarrel))
  (CallFunction|InitialiseHealthbarWidget))

(fn ConstructionScript)

(fn InitialiseHealthbarWidget
  (bind _ashealthbar_bp (Utilities|Casting|CastToHealthbar_BP (UserInterface|GetUserWidgetObject (Variables|Default|GetWidget))))
  (Variables|/Game/UI/Healthbar_BP.Healthbar_BP_C|SetTank _ashealthbar_bp self)
  (return))